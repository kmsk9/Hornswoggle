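; AI controller for enemies that runs the BT_Enemy behavior tree on the BB_Enemy blackboard when it possesses a pawn.
; On BeginPlay it stores the player character in the blackboard as Enemy.
; Perception updates for the player set canSeePlayer from the first last-sensed stimulus.
; When sensing fails, it saves the player's current position as LastSeenLocation and draws a red debug sphere there.
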(event `self.OnPossess`
  (params (PossessedPawn :type "Pawn Object Reference"))
  (`self.UseBlackboard` "/Game/Blueprints/AI/BB_Enemy.BB_Enemy")
  (`self.RunBehaviorTree` "/Game/Blueprints/AI/BT_Enemy.BT_Enemy"))

(event `self.ReceiveBeginPlay`
  (bind _output_get (set `self.Enemy` (`GameplayStatics.GetPlayerCharacter` 0)))
  (`BlackboardComponent.SetValueAsObject` (`AIBlueprintHelperLibrary.GetBlackboard` null) "Enemy" _output_get))

(event `self.AIPerception.OnPerceptionUpdated`
  (params (UpdatedActors :type "Array of Actor Object Reference"))
  (bind _returnvalue (`AIBlueprintHelperLibrary.GetBlackboard` null))
  (bind _returnvalue_2 (`self.K2_GetActorLocation` (`self.Enemy`)))
  (for _array_element UpdatedActors
    (if (== _array_element (`self.Enemy`))
      (bind _info (`AIPerceptionComponent.GetActorsPerception` (`self.AIPerception`) _array_element))
      (bind (_age _expirationage _strength _stimuluslocation _receiverlocation _tag _bsuccessfullysensed) (break `AIStimulus` (`|GetArrayItem` (`.LastSensedStimuli` (break `ActorPerceptionBlueprintInfo` _info)))))
      (`BlackboardComponent.SetValueAsBool` _returnvalue "canSeePlayer" _bsuccessfullysensed)
      (if (not _bsuccessfullysensed)
        (`BlackboardComponent.SetValueAsVector` _returnvalue "LastSeenLocation" _returnvalue_2)
        (`KismetSystemLibrary.DrawDebugSphere` _returnvalue_2 100.0 12 (struct :`R` 1.0 :`A` 1.0) 5.0 1.0)))))

(fn `UserConstructionScript`)