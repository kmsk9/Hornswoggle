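; Behavior tree task for AI_Enemy_2 that picks a location to search, based on where its Enemy is.
; It averages the positions of the Blackboard's Enemy actor and the controlled pawn, then takes a random reachable navmesh point within a fixed radius of that midpoint.
; The result is written to the SearchLocation key and the task finishes successfully.
; If the pawn is not an AI_Enemy_2, the task never calls FinishExecute.
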(event `self.ReceiveExecuteAI`
  (params (OwnerController :type "AIController Object Reference") (ControlledPawn :type "Pawn Object Reference"))
  (bind _returnvalue (`AIBlueprintHelperLibrary.GetBlackboard` OwnerController))
  (bind (_returnvalue_x _returnvalue_y _returnvalue_z) (`KismetMathLibrary.BreakVector` (`Actor.K2_GetActorLocation` (cast `Actor` (`BlackboardComponent.GetValueAsObject` _returnvalue "Enemy") :!pure true))))
  (bind _asai_enemy_2 (cast `/Game/Blueprints/AI/AI_Enemy_2` ControlledPawn))
  (`BlackboardComponent.SetValueAsVector` _returnvalue "SearchLocation" (`NavigationSystem.K2_GetRandomReachablePointInRadius` (/ (+ (`KismetMathLibrary.MakeVector` _returnvalue_x _returnvalue_y _returnvalue_z) (`KismetMathLibrary.MakeVector` (.x (`Actor.K2_GetActorLocation` _asai_enemy_2)) (.y (`Actor.K2_GetActorLocation` _asai_enemy_2)) (.z (`Actor.K2_GetActorLocation` _asai_enemy_2)))) 2.0) 2000.0))
  (`self.FinishExecute` true))