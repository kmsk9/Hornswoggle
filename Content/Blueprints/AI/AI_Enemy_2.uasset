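; AI enemy that fires cannonballs at the player and drops gold on death, likely a ship given its weapons.
; A front trigger sets CanAttackFront, gating the externally called ShootEnemy spawn.
; Overlapping player projectiles and barrels subtract health scaled from player damage, with bar shot also briefly slowing movement.
; Tick prints debug state and handles death, incrementing the player's kill counter during Mission01.
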(event `self.shootFront.OnComponentBeginOverlap`
  (params (OverlappedComponent :type "PrimitiveComponent Object Reference") (OtherActor :type "Actor Object Reference") (OtherComp :type "PrimitiveComponent Object Reference") (OtherBodyIndex :type Integer) (bFromSweep :type Boolean) (SweepResult :type "HitResult Structure (by ref)"))
  (cast `/Game/Blueprints/Player/Player_BP_Redo` OtherActor)
  (set `self.canAttackFront` true))

(event `self.shootFront.OnComponentEndOverlap`
  (params (OverlappedComponent :type "PrimitiveComponent Object Reference") (OtherActor :type "Actor Object Reference") (OtherComp :type "PrimitiveComponent Object Reference") (OtherBodyIndex :type Integer))
  (cast `/Game/Blueprints/Player/Player_BP_Redo` OtherActor)
  (set `self.canAttackFront` false))

(event `self.ReceiveBeginPlay`
  (bind _asplayer_bp_redo (cast `/Game/Blueprints/Player/Player_BP_Redo` (`GameplayStatics.GetPlayerCharacter` 0))))

(event `self.ReceiveActorBeginOverlap`
  (params (OtherActor :type "Actor Object Reference"))
  (bind _charactermovement (`self.CharacterMovement`))
  (`|ExecutionSequence`
    (:`then_0`
      (cast `/Game/Blueprints/Player/Ammo/CannonBall_BP` OtherActor)
      (bind _damage (`/Game/Blueprints/Player/Player_BP_Redo.Damage` (stale `self.ReceiveBeginPlay` _asplayer_bp_redo)))
      (set `self.Health` (- (`self.Health`) _damage)))
    (:`then_1`
      (cast `/Game/Blueprints/Player/Ammo/CannonBall_BP1` OtherActor)
      (set `self.Health` (- (`self.Health`) _damage)))
    (:`then_2`
      (cast `/Game/Blueprints/Player/Ammo/ExplosiveShot_BP` OtherActor)
      (set `self.Health` (- (`self.Health`) (* _damage 3.0))))
    (:`then_3`
      (cast `/Game/Blueprints/Player/Ammo/ExplosiveShot_BP1` OtherActor)
      (set `self.Health` (- (`self.Health`) (* _damage 3.0))))
    (:`then_4`
      (cast `/Game/Blueprints/Player/Ammo/BarShot_BP` OtherActor)
      (set `self.Health` (- (`self.Health`) _damage))
      (set `CharacterMovementComponent.MaxWalkSpeed` 150.0 _charactermovement :!label _label)
      (`KismetSystemLibrary.Delay` 3.0)
      (set `CharacterMovementComponent.MaxWalkSpeed` 400.0 _charactermovement))
    (:`then_5`
      (cast `/Game/Blueprints/Player/Ammo/BarShot_BP1` OtherActor)
      (set `self.Health` (- (`self.Health`) _damage))
      (goto _label))
    (:`then_6`
      (cast `/Game/Blueprints/Player/Ammo/Barrel_BP` OtherActor)
      (set `self.Health` (- (`self.Health`) (* _damage 5.0))))))

(event `self.ReceiveTick`
  (params (DeltaSeconds :type "Float (single-precision)"))
  (`|ExecutionSequence`
    (:`then_0`
      (`KismetSystemLibrary.PrintString` (`KismetStringLibrary.Conv_BoolToString` (`self.canAttackFront`))))
    (:`then_1`
      (if (<= (`self.Health`) 0.0)
        (bind _asplayer_bp_redo (cast `/Game/Blueprints/Player/Player_BP_Redo` (`GameplayStatics.GetPlayerPawn` 0)))
        (if (`/Game/Blueprints/Player/Player_BP_Redo.Mission_01` _asplayer_bp_redo)
          (set `/Game/Blueprints/Player/Player_BP_Redo.BSKilledActive` (+ (`/Game/Blueprints/Player/Player_BP_Redo.BSKilledActive` _asplayer_bp_redo) 1) _asplayer_bp_redo))
        (`self.K2_DestroyActor`)
        (`|SpawnActorFromClass` "/Game/Blueprints/Extras/Gold_BP.Gold_BP_C" (`self.GetTransform`) "Undefined" "OverrideRootScale")))))

(event `ShootEnemy`
  (params (`Enemy to Shoot` :type "Actor Object Reference"))
  (bind (_returnvalue_location _returnvalue_rotation) (`KismetMathLibrary.BreakTransform` (`SceneComponent.K2_GetComponentToWorld` (`self.Front`))))
  (if (`self.canAttackFront`)
    (`|SpawnActorFromClass` "/Game/Blueprints/AI/AI_CannonBall_BP1.AI_CannonBall_BP1_C" (`KismetMathLibrary.MakeTransform` _returnvalue_location _returnvalue_rotation (4.0 4.0 4.0)) "Undefined" "OverrideRootScale")
    (`KismetSystemLibrary.PrintString` "Hello")))

(fn `UserConstructionScript`)