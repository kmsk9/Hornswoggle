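; AI controller for the AI_Enemy_2 pawn that runs BT_Enemy on BB_Enemy when it possesses a pawn.
; BeginPlay seeds the blackboard with the player character as Enemy and the pawn's starting position as myLocation.
; Perception updates set canSeePlayer from the player's first sensed stimulus.
; When sensing fails, it records the player's position as LastSeenLocation, with a debug sphere and printed state for debugging.
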(event `self.OnPossess`
  (params (PossessedPawn :type "Pawn Object Reference"))
  (`self.UseBlackboard` "/Game/Blueprints/AI/BB_Enemy.BB_Enemy")
  (`self.RunBehaviorTree` "/Game/Blueprints/AI/BT_Enemy.BT_Enemy"))

(event `self.ReceiveBeginPlay`
  (bind _returnvalue (`AIBlueprintHelperLibrary.GetBlackboard` null))
  (`|ExecutionSequence`
    (:`then_0`
      (bind _output_get (set `self.Enemy` (`GameplayStatics.GetPlayerCharacter` 0)))
      (`BlackboardComponent.SetValueAsObject` _returnvalue "Enemy" _output_get))
    (:`then_1`
      (bind _asai_enemy_2 (cast `/Game/Blueprints/AI/AI_Enemy_2` (`self.K2_GetPawn`)))
      (`BlackboardComponent.SetValueAsVector` _returnvalue "myLocation" (`self.K2_GetActorLocation` _asai_enemy_2)))))

(event `self.AIPerception.OnPerceptionUpdated`
  (params (UpdatedActors :type "Array of Actor Object Reference"))
  (bind _returnvalue (`AIBlueprintHelperLibrary.GetBlackboard` null))
  (bind _returnvalue_2 (`self.K2_GetActorLocation` (`self.Enemy`)))
  (for _array_element UpdatedActors
    (if (== _array_element (`self.Enemy`))
      (bind _info (`AIPerceptionComponent.GetActorsPerception` (`self.AIPerception`) _array_element))
      (bind (_age _expirationage _strength _stimuluslocation _receiverlocation _tag _bsuccessfullysensed) (break `AIStimulus` (`|GetArrayItem` (`.LastSensedStimuli` (break `ActorPerceptionBlueprintInfo` _info)))))
      (`BlackboardComponent.SetValueAsBool` _returnvalue "canSeePlayer" _bsuccessfullysensed)
      (`KismetSystemLibrary.PrintString` (`KismetStringLibrary.Conv_BoolToString` (`BlackboardComponent.GetValueAsBool` (`AIBlueprintHelperLibrary.GetBlackboard` null) "canSeePlayer")))
      (if (not _bsuccessfullysensed)
        (`BlackboardComponent.SetValueAsVector` _returnvalue "LastSeenLocation" _returnvalue_2)
        (`KismetSystemLibrary.DrawDebugSphere` _returnvalue_2 100.0 12 (struct :`R` 1.0 :`A` 1.0) 5.0 1.0)))))

(fn `UserConstructionScript`)