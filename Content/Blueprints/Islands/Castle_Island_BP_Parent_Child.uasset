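; Child island Blueprint for the castle island that tells the player when they are within docking range.
; Overlapping its DockArea component clears the player's AtSea flag, allows main island docking and sets CurrentIsland to this island's hard-coded index.
; Leaving the area restores the at-sea state, disables docking and resets the island index.
; The construction script only calls the parent's.
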(event `self.DockArea.OnComponentBeginOverlap`
  (params (OverlappedComponent :type "PrimitiveComponent Object Reference") (OtherActor :type "Actor Object Reference") (OtherComp :type "PrimitiveComponent Object Reference") (OtherBodyIndex :type Integer) (bFromSweep :type Boolean) (SweepResult :type "HitResult Structure (by ref)"))
  (bind _asplayer_bp_redo (cast `/Game/Blueprints/Player/Player_BP_Redo` OtherActor))
  (set `/Game/Blueprints/Player/Player_BP_Redo.atSea` false _asplayer_bp_redo)
  (set `/Game/Blueprints/Player/Player_BP_Redo.CanDockMainIsland` true _asplayer_bp_redo)
  (set `/Game/Blueprints/Player/Player_BP_Redo.CurrentIsland` 2 _asplayer_bp_redo))

(event `self.DockArea.OnComponentEndOverlap`
  (params (OverlappedComponent :type "PrimitiveComponent Object Reference") (OtherActor :type "Actor Object Reference") (OtherComp :type "PrimitiveComponent Object Reference") (OtherBodyIndex :type Integer))
  (bind _asplayer_bp_redo (cast `/Game/Blueprints/Player/Player_BP_Redo` OtherActor))
  (set `/Game/Blueprints/Player/Player_BP_Redo.atSea` true _asplayer_bp_redo)
  (set `/Game/Blueprints/Player/Player_BP_Redo.CanDockMainIsland` false _asplayer_bp_redo)
  (set `/Game/Blueprints/Player/Player_BP_Redo.CurrentIsland` 0 _asplayer_bp_redo))

(fn `UserConstructionScript`
  (`parent.UserConstructionScript`))