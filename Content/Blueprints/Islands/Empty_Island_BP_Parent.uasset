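; Parent Blueprint for empty islands that the player can dock at.
; Overlapping the DockingDisplay volume shows the Widget component to signal docking, and leaving it hides the widget.
; Overlapping the DockArea volume clears the player's AtSea flag and enables CanDockEmptyIsland, and leaving it reverses both.
; Both volumes respond only to Player_BP_Redo, and the docking action itself is not handled here.
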(event `self.DockingDisplay.OnComponentBeginOverlap`
  (params (OverlappedComponent :type "PrimitiveComponent Object Reference") (OtherActor :type "Actor Object Reference") (OtherComp :type "PrimitiveComponent Object Reference") (OtherBodyIndex :type Integer) (bFromSweep :type Boolean) (SweepResult :type "HitResult Structure (by ref)"))
  (cast `/Game/Blueprints/Player/Player_BP_Redo` OtherActor)
  (`SceneComponent.SetVisibility` (`self.Widget`) true false))

(event `self.DockingDisplay.OnComponentEndOverlap`
  (params (OverlappedComponent :type "PrimitiveComponent Object Reference") (OtherActor :type "Actor Object Reference") (OtherComp :type "PrimitiveComponent Object Reference") (OtherBodyIndex :type Integer))
  (cast `/Game/Blueprints/Player/Player_BP_Redo` OtherActor)
  (`SceneComponent.SetVisibility` (`self.Widget`) false false))

(event `self.DockArea.OnComponentBeginOverlap`
  (params (OverlappedComponent :type "PrimitiveComponent Object Reference") (OtherActor :type "Actor Object Reference") (OtherComp :type "PrimitiveComponent Object Reference") (OtherBodyIndex :type Integer) (bFromSweep :type Boolean) (SweepResult :type "HitResult Structure (by ref)"))
  (bind _asplayer_bp_redo (cast `/Game/Blueprints/Player/Player_BP_Redo` OtherActor))
  (set `/Game/Blueprints/Player/Player_BP_Redo.atSea` false _asplayer_bp_redo)
  (set `/Game/Blueprints/Player/Player_BP_Redo.CanDockEmptyIsland` true _asplayer_bp_redo))

(event `self.DockArea.OnComponentEndOverlap`
  (params (OverlappedComponent :type "PrimitiveComponent Object Reference") (OtherActor :type "Actor Object Reference") (OtherComp :type "PrimitiveComponent Object Reference") (OtherBodyIndex :type Integer))
  (bind _asplayer_bp_redo (cast `/Game/Blueprints/Player/Player_BP_Redo` OtherActor))
  (set `/Game/Blueprints/Player/Player_BP_Redo.atSea` true _asplayer_bp_redo)
  (set `/Game/Blueprints/Player/Player_BP_Redo.CanDockEmptyIsland` false _asplayer_bp_redo))

(fn `UserConstructionScript`)