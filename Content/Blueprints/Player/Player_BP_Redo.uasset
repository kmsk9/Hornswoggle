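; Player pirate ship with force-based movement, yaw steering, four selectable weapons, upgradeable hull and sail meshes, and HUD, dock menu and map widgets.
; Tick drives scurvy, sail visuals, mission checks, cursor-led camera and MiniCams.
; Cannon, bar and explosive shots fire only when tick-computed facing and aim quadrants match; barrels drop freely.
; Overlaps apply damage or collect gold; death respawns at a checkpoint, leaving a lootable shipwreck.
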(event `HullLevelUp`
  ;[1 1 1] Hull Level up static mesh changer
  (if (== (`self.HullLevel`) (`self.HullLevel_02_amount`))
    (`StaticMeshComponent.SetStaticMesh` (`self.Hull`) "/Game/Art/ShipMeshes/Pirates_Ship_Hull_Level_02.Pirates_Ship_Hull_Level_02")
    (elif (== (`self.HullLevel`) (`self.HullLevel_03_amount`))
      (`StaticMeshComponent.SetStaticMesh` (`self.Hull`) "/Game/Art/ShipMeshes/Pirates_Ship_Hull_Level_03.Pirates_Ship_Hull_Level_03"))))

(event `self.ReceiveBeginPlay`
  ;[0.1969 0 1] Setting HUD on begin
  (set `PlayerController.bShowMouseCursor` true (`GameplayStatics.GetPlayerController` 0))
  (bind _returnvalue (`|CreateWidget` "/Game/Blueprints/UI/HUD.HUD_C"))
  (`UserWidget.AddToViewport` _returnvalue 0)
  (set `PlayerController.CurrentMouseCursor` "Crosshairs" (`GameplayStatics.GetPlayerController` 0)))

(event `self.ReceiveActorBeginOverlap`
  (params (OtherActor :type "Actor Object Reference"))
  ;[1 0 0.8197] Event Overlap
  (`|ExecutionSequence`
    (:`then_0`
      ;;[0 1 0.09028] Damage
      ;;;[1 1 1] CannonBall Damage
      (if (`self.canBeDamaged`)
        (cast `/Game/Blueprints/AI/AI_CannonBall_BP1` OtherActor)
        (set `self.Health` (- (`self.Health`) 5.0))
        (set `self.canBeDamaged` false :!label _label)
        (`KismetSystemLibrary.Delay` 0.2)
        (set `self.canBeDamaged` true)))
    (:`then_1`
      ;;;[1 1 1] Rocks Damage
      (cast `/Game/Blueprints/IslandsHazards/Rocks` OtherActor)
      (set `self.Health` (- (`self.Health`) 25.0))
      (goto _label))
    (:`then_2`
      ;;[1 1 1] Gold
      (bind _asgold_bp (cast `/Game/Blueprints/Extras/Gold_BP` OtherActor))
      (set `self.Gold` (+ (`self.Gold`) 100.0))
      (`self.K2_DestroyActor` _asgold_bp))
    (:`then_3`
      ;;[1 1 1] Shipwreck
      (bind _asshipwreck (cast `/Game/Blueprints/Extras/Shipwreck` OtherActor))
      (set `self.Gold` (+ (`self.Gold`) (`self.GoldonDed`)))
      (`self.K2_DestroyActor` _asshipwreck))))

(event `Key|One`
  (params (Key :type "Key Structure" :default "AnyKey"))
  ;[0 0.475 0.4112] Weapon Change
  (:`Pressed`
    (set `self.WeaponSelect` 1)))

(event `InputAxis|Move`
  (params (AxisValue :type "Float (single-precision)"))
  (bind (_returnvalue_roll _returnvalue_pitch _returnvalue_yaw) (`KismetMathLibrary.BreakRotator` (`SceneComponent.K2_GetComponentRotation` (`self.Scene`))))
  ;[0 0.02183 1] Movement
  (`PrimitiveComponent.AddForce` (`self.CapsuleComponent`) (* (* (`KismetMathLibrary.GetForwardVector` (`KismetMathLibrary.MakeRotator` _returnvalue_roll _returnvalue_pitch (+ _returnvalue_yaw 90.0))) AxisValue) (`self.Speed`)) "None" false))

(event `Key|Two`
  (params (Key :type "Key Structure" :default "AnyKey"))
  ;[0 0.475 0.4112] Weapon Change
  (:`Pressed`
    (set `self.WeaponSelect` 2)))

(event `Key|Three`
  (params (Key :type "Key Structure" :default "AnyKey"))
  ;[0 0.475 0.4112] Weapon Change
  (:`Pressed`
    (set `self.WeaponSelect` 3)))

(event `Key|Four`
  (params (Key :type "Key Structure" :default "AnyKey"))
  ;[0 0.475 0.4112] Weapon Change
  (:`Pressed`
    (set `self.WeaponSelect` 4)))

(event `InputAxis|Rotate`
  (params (AxisValue :type "Float (single-precision)"))
  (bind _returnvalue (* AxisValue (`GameplayStatics.GetWorldDeltaSeconds`) (`self.RotateSpeed`)))
  ;[0 0.02183 1] Movement
  (`|ExecutionSequence`
    (:`then_0`
      (`SceneComponent.K2_AddWorldRotation` (`self.Scene`) (`KismetMathLibrary.MakeRotator` 0.0 0.0 _returnvalue) false false))
    (:`then_1`
      (`SceneComponent.K2_AddWorldRotation` (`self.Scene`) (`KismetMathLibrary.MakeRotator` 0.0 0.0 _returnvalue) false false))))

(event `Key|E`
  (params (Key :type "Key Structure" :default "AnyKey"))
  (bind _returnvalue (`GameplayStatics.GetPlayerController` 0))
  (bind _returnvalue_2 (`GameplayStatics.GetPlayerController` 0))
  ;[0.2121 1 0] Open Menu
  (:`Pressed`
    (if (`self.CanDockMainIsland`)
      (bind _returnvalue_3 (`|CreateWidget` "/Game/Blueprints/UI/Main_Island_MainMenuUI.Main_Island_MainMenuUI_C" (`GameplayStatics.GetPlayerController` 0)))
      (`UserWidget.AddToViewport` _returnvalue_3 0)
      (`WidgetBlueprintLibrary.SetInputMode_UIOnlyEx` _returnvalue_2)
      (set `PlayerController.CurrentMouseCursor` "Default" _returnvalue_2)
      (elif (`self.CanDockEmptyIsland`)
        (bind _returnvalue_4 (`|CreateWidget` "/Game/Blueprints/UI/Empty_Island_MainMenuUI.Empty_Island_MainMenuUI_C" (`GameplayStatics.GetPlayerController` 0)))
        (`UserWidget.AddToViewport` _returnvalue_4 0)
        (`WidgetBlueprintLibrary.SetInputMode_UIOnlyEx` _returnvalue)
        (set `PlayerController.CurrentMouseCursor` "Default" _returnvalue)))))

(event `Mission_01_Active`
  ;[1 0.9228 0] Missions
  (if (== (`self.BSKilledActive`) 2)
    (`self.Mission_01_Completed`)))

(event `Mission_01_Completed`
  ;[1 0.9228 0] Missions
  (set `self.Mission_01` false)
  (set `self.BSKilledActive` 0)
  (bind _returnvalue (`|CreateWidget` "/Game/Blueprints/UI/Missions_01_Complete.Missions_01_Complete_C" (`GameplayStatics.GetPlayerController` 0)))
  (`UserWidget.AddToViewport` _returnvalue 0))

(event `Mission_02_Completed`
  ;[1 0.9228 0] Missions
  (set `self.Mission_02` false)
  (bind _returnvalue (`|CreateWidget` "/Game/Blueprints/UI/Missions_02_Complete.Missions_02_Complete_C" (`GameplayStatics.GetPlayerController` 0)))
  (`UserWidget.AddToViewport` _returnvalue 0))

(event `Key|MouseScrollDown`
  (params (Key :type "Key Structure" :default "AnyKey"))
  (bind _springarm (`self.SpringArm`))
  ;[1 1 1] Cam zoom
  (:`Pressed`
    (set `SpringArmComponent.TargetArmLength` (`KismetMathLibrary.FClamp` (+ (`SpringArmComponent.TargetArmLength` _springarm) 500.0) 5000.0 15000.0) _springarm)))

(event `self.ReceiveTick`
  (params (DeltaSeconds :type "Float (single-precision)"))
  (bind _cursor (`self.Cursor`))
  (bind (_returnvalue_roll _returnvalue_pitch _returnvalue_yaw) (`KismetMathLibrary.BreakRotator` (`SceneComponent.K2_GetComponentRotation` (`self.Scene`))))
  (bind (_returnvalue_roll_2 _returnvalue_pitch_2 _returnvalue_yaw_2) (`KismetMathLibrary.BreakRotator` (`SceneComponent.K2_GetComponentRotation` (`self.Tip`))))
  (bind (_returnvalue_roll_3 _returnvalue_pitch_3 _returnvalue_yaw_3) (`KismetMathLibrary.BreakRotator` (`SceneComponent.K2_GetComponentRotation` (`self.Scene`))))
  (bind (_returnvalue_roll_4 _returnvalue_pitch_4 _returnvalue_yaw_4) (`KismetMathLibrary.BreakRotator` (`SceneComponent.K2_GetComponentRotation` (`self.Tip`))))
  (bind (_returnvalue_roll_5 _returnvalue_pitch_5 _returnvalue_yaw_5) (`KismetMathLibrary.BreakRotator` (`SceneComponent.K2_GetComponentRotation` (`self.Scene`))))
  (bind (_returnvalue_roll_6 _returnvalue_pitch_6 _returnvalue_yaw_6) (`KismetMathLibrary.BreakRotator` (`SceneComponent.K2_GetComponentRotation` (`self.Scene`))))
  (bind (_returnvalue_roll_7 _returnvalue_pitch_7 _returnvalue_yaw_7) (`KismetMathLibrary.BreakRotator` (`SceneComponent.K2_GetComponentRotation` (`self.Tip`))))
  (bind (_returnvalue_roll_8 _returnvalue_pitch_8 _returnvalue_yaw_8) (`KismetMathLibrary.BreakRotator` (`SceneComponent.K2_GetComponentRotation` (`self.Tip`))))
  (bind (_relativelocation_x _relativelocation_y) (`KismetMathLibrary.BreakVector` (`SceneComponent.RelativeLocation` _cursor)))
  (bind (_bblockinghit _binitialoverlap _time _location _impactpoint _normal _impactnormal) (`GameplayStatics.BreakHitResult` (`PlayerController.GetHitResultUnderCursorByChannel` (`GameplayStatics.GetPlayerController` 0) "TraceTypeQuery1" true)))
  ;[1 0.448 0] Event Tick
  (`|ExecutionSequence`
    (:`then_0`
      ;;[1 1 1] Scurvy
      (if (`self.atSea`)
        (`KismetSystemLibrary.Delay` 3.0)
        (set `self.Scurvy` (+ (`self.Scurvy`) 1.0))))
    (:`then_1`
      ;;[1 1 1] Death
      (if (<= (`self.Health`) 0.0)
        (set `self.DeathPoint` (`self.K2_GetActorLocation`))
        (set `self.isDead` true)
        (set `self.GoldonDed` (`self.Gold`))
        (set `self.Gold` 0.0)
        (`self.K2_SetActorLocation` (`self.Checkpoint`))
        (set `self.Health` 100.0)))
    (:`then_2`
      ;;[1 1 1] Set Death Point
      (if (`self.isDead`)
        (`|SpawnActorFromClass` "/Game/Blueprints/Extras/Shipwreck.Shipwreck_C" (`KismetMathLibrary.MakeTransform` (`self.DeathPoint`)) "Undefined" "OverrideRootScale")
        (set `self.isDead` false)))
    (:`then_3`
      ;;[1 1 1] Mission Active
      (if (`self.Mission_01`)
        (`self.Mission_01_Active`)))
    (:`then_4`
      ;;[1 1 1] Set Missing Health
      (set `self.MissingHealth` (* (- (`self.Health`) 100.0) -1.0)))
    (:`then_5`
      ;;[1 1 1] Setting Dock/AtSea static mesh
      (if (`self.atSea`)
        (if (< (`self.SailsLevel`) (`self.SailLevel_02_amount`))
          (`StaticMeshComponent.SetStaticMesh` (`self.Sails`) "/Game/Art/ShipMeshes/Pirates_Ship_Level_01_SailsDown.Pirates_Ship_Level_01_SailsDown")
          (`SceneComponent.K2_SetRelativeLocation` (`self.Sails`) (-43.0 -107.0 -500.0) false false)
          (elif (< (`self.SailsLevel`) (`self.SailLevel_03_amount`))
            (`StaticMeshComponent.SetStaticMesh` (`self.Sails`) "/Game/Art/ShipMeshes/Pirates_Ship_Level_02_SailsDown.Pirates_Ship_Level_02_SailsDown")
            (elif (> (`self.SailsLevel`) (`self.SailLevel_03_amount`))
              (`StaticMeshComponent.SetStaticMesh` (`self.Sails`) "/Game/Art/ShipMeshes/Pirates_Ship_Level_03_SailsDown.Pirates_Ship_Level_03_SailsDown"))))
        (elif (< (`self.SailsLevel`) (`self.SailLevel_02_amount`))
          (`StaticMeshComponent.SetStaticMesh` (`self.Sails`) "/Game/Art/ShipMeshes/Pirates_Ship_Level_01_SailsUp.Pirates_Ship_Level_01_SailsUp")
          (elif (< (`self.SailsLevel`) (`self.SailLevel_03_amount`))
            (`StaticMeshComponent.SetStaticMesh` (`self.Sails`) "/Game/Art/ShipMeshes/Pirates_Ship_Level_02_SailsUp.Pirates_Ship_Level_02_SailsUp")
            (elif (> (`self.SailsLevel`) (`self.SailLevel_03_amount`))
              (`StaticMeshComponent.SetStaticMesh` (`self.Sails`) "/Game/Art/ShipMeshes/Pirates_Ship_Level_03_SailsUp.Pirates_Ship_Level_03_SailsUp"))))))
    (:`then_6`
      ;;[1 1 1] Aim
      (if (or (and (>= _returnvalue_yaw_4 90.0) (<= _returnvalue_yaw_4 180.0)) (and (>= _returnvalue_yaw_4 -180.0) (<= _returnvalue_yaw_4 -90.0)))
        (set `self.aimDown` true)
        (else
          (set `self.aimDown` false))))
    (:`then_7`
      (if (and (>= _returnvalue_yaw_3 -135.0) (<= _returnvalue_yaw_3 -40.0))
        (set `self.faceDown` true)
        (else
          (set `self.faceDown` false))))
    (:`then_8`
      (if (and (>= _returnvalue_yaw_6 -45.0) (<= _returnvalue_yaw_6 45.0))
        (set `self.faceLeft` true)
        (else
          (set `self.faceLeft` false))))
    (:`then_9`
      (if (and (>= _returnvalue_yaw_7 -180.0) (<= _returnvalue_yaw_7 0.0))
        (set `self.AimLeft` true)
        (else
          (set `self.AimLeft` false))))
    (:`then_10`
      (if (or (and (>= _returnvalue_yaw 135.0) (<= _returnvalue_yaw 180.0)) (and (>= _returnvalue_yaw -180.0) (<= _returnvalue_yaw -135.0)))
        (set `self.faceRight` true)
        (else
          (set `self.faceRight` false))))
    (:`then_11`
      (if (and (>= _returnvalue_yaw_2 0.0) (<= _returnvalue_yaw_2 180.0))
        (set `self.AimRight` true)
        (else
          (set `self.AimRight` false))))
    (:`then_12`
      (if (and (<= _returnvalue_yaw_8 90.0) (>= _returnvalue_yaw_8 -90.0))
        (set `self.aimUP` true)
        (else
          (set `self.aimUP` false))))
    (:`then_13`
      (if (and (>= _returnvalue_yaw_5 40.0) (<= _returnvalue_yaw_5 135.0))
        (set `self.faceUP` true)
        (else
          (set `self.faceUP` false))))
    (:`then_14`
      ;;[1 1 1] Cam moving
      (`SceneComponent.K2_SetWorldLocationAndRotation` _cursor _location (`KismetMathLibrary.MakeRotationFromAxes` _impactnormal) false false)
      (`SceneComponent.K2_SetRelativeLocation` (`self.Cam`) (`KismetMathLibrary.MakeVector` (/ _relativelocation_x 5.0) (/ _relativelocation_y 5.0)) false false))
    (:`then_15`
      (bind _outactors (`GameplayStatics.GetAllActorsOfClass` "/Game/Blueprints/MiniMap/MiniCam.MiniCam_C"))
      (for _array_element _outactors
        (`/Game/Blueprints/MiniMap/MiniCam.OutSideTick` _array_element)))))

(event `Key|MouseScrollUp`
  (params (Key :type "Key Structure" :default "AnyKey"))
  (bind _springarm (`self.SpringArm`))
  ;[1 1 1] Cam zoom
  (:`Pressed`
    (set `SpringArmComponent.TargetArmLength` (`KismetMathLibrary.FClamp` (- (`SpringArmComponent.TargetArmLength` _springarm) 500.0) 5000.0 15000.0) _springarm)))

(event `Key|L`
  (params (Key :type "Key Structure" :default "AnyKey"))
  (:`Pressed`
    (if (`self.MiniMap`)
      (bind _returnvalue (`|CreateWidget` "/Game/Blueprints/UI/MapUi.MapUi_C"))
      (`UserWidget.AddToViewport` _returnvalue 0)
      (set `self.MiniMap` false)
      (else
        (`Widget.RemoveFromParent` _returnvalue)
        (set `self.MiniMap` true)))))

(event `InputAction|Shoot`
  (params (Key :type "Key Structure" :default "AnyKey"))
  ;[1 0 0] Shooting
  (:`Pressed`
    (`|ExecutionSequence`
      (:`then_0`
        (if (== (`self.WeaponSelect`) 1)
          (`self.CannonShot`)
          (`KismetSystemLibrary.Delay` 0.5)
          (set `self.Can_Fire_Cannon` true)))
      (:`then_1`
        (if (== (`self.WeaponSelect`) 2)
          (`self.BarShot`)
          (`KismetSystemLibrary.Delay` 2.0)
          (set `self.Can_Fire_Bar` true)))
      (:`then_2`
        (if (== (`self.WeaponSelect`) 3)
          (`self.ExplosiveShot`)
          (`KismetSystemLibrary.Delay` 0.3)
          (set `self.Can_FIre_Explosive` true)))
      (:`then_3`
        (if (== (`self.WeaponSelect`) 4)
          (`self.Barrel`)
          (`KismetSystemLibrary.Delay` 4.0)
          (set `self.Can_Fire_Barrel` true))))))

(event `Key|K`
  (params (Key :type "Key Structure" :default "AnyKey"))
  ;[1 1 1] Uping Hull Level for test
  (:`Pressed`
    (set `self.HullLevel` (+ (`self.HullLevel`) 1))
    (`self.HullLevelUp`)))

(event `Key|J`
  (params (Key :type "Key Structure" :default "AnyKey"))
  ;[1 1 1] Uping Sails level for test
  (:`Pressed`
    (set `self.SailsLevel` (+ (`self.SailsLevel`) 1))))

(fn `Barrel`
  (bind _returnvalue_location (`KismetMathLibrary.BreakTransform` (`SceneComponent.K2_GetComponentToWorld` (`self.Drop`))))
  (if (`self.Can_Fire_Barrel`)
    (`|SpawnActorFromClass` "/Game/Blueprints/Player/Ammo/Barrel_BP.Barrel_BP_C" (`KismetMathLibrary.MakeTransform` _returnvalue_location (struct :`Pitch` 90.0) (2.0 2.0 2.0)) "Undefined" "OverrideRootScale")
    (set `self.Can_Fire_Barrel` false)))

(fn `BarShot`
  (bind (_relativerotation_roll _relativerotation_pitch _relativerotation_yaw) (`KismetMathLibrary.BreakRotator` (`SceneComponent.RelativeRotation` (`self.AimArrow`))))
  (bind (_returnvalue_roll _returnvalue_pitch _returnvalue_yaw) (`KismetMathLibrary.BreakRotator` (`KismetMathLibrary.MakeRotFromX` (`KismetMathLibrary.Normal` (- (`.Location` (`GameplayStatics.BreakHitResult` (`PlayerController.GetHitResultUnderCursorByChannel` (`GameplayStatics.GetPlayerController` 0) "TraceTypeQuery1" true))) (`self.K2_GetActorLocation`))))))
  (if (`self.Can_Fire_Bar`)
    (`SceneComponent.K2_SetWorldRotation` (`self.AimArrow`) (`KismetMathLibrary.MakeRotator` 0.0 0.0 _returnvalue_yaw) false false)
    (`|ExecutionSequence`
      (:`then_0`
        (if (and (`self.faceUP`) (`self.aimUP`))
          (if (or (`self.faceDown`) (`self.faceLeft`) (`self.faceRight`))
            (set `self.Can_Fire_Cannon` false)
            (else
              (`|SpawnActorFromClass` "/Game/Blueprints/Player/Ammo/BarShot_BP.BarShot_BP_C" (`KismetMathLibrary.MakeTransform` (`SceneComponent.K2_GetComponentLocation` (`self.AimArrow`)) (`KismetMathLibrary.MakeRotator` 0.0)) "Undefined" "OverrideRootScale" :!label _label)
              (set `self.Can_Fire_Bar` false)
              (if (>= _relativerotation_yaw -90.0)
                (`ActorComponent.Activate` (`self.RightPart`) true)
                (else
                  (`ActorComponent.Activate` (`self.LeftPart`) true)))))))
      (:`then_1`
        (if (and (`self.aimDown`) (`self.faceDown`))
          (goto _label)))
      (:`then_2`
        (if (and (`self.faceLeft`) (`self.AimLeft`))
          (goto _label)))
      (:`then_3`
        (if (and (`self.faceRight`) (`self.AimRight`))
          (goto _label))))))

(fn `CannonShot`
  (bind (_returnvalue_roll _returnvalue_pitch _returnvalue_yaw) (`KismetMathLibrary.BreakRotator` (`SceneComponent.K2_GetComponentRotation` (`self.Tip`))))
  (bind (_relativerotation_roll _relativerotation_pitch _relativerotation_yaw) (`KismetMathLibrary.BreakRotator` (`SceneComponent.RelativeRotation` (`self.AimArrow`))))
  (bind (_returnvalue_roll_2 _returnvalue_pitch_2 _returnvalue_yaw_2) (`KismetMathLibrary.BreakRotator` (`KismetMathLibrary.MakeRotFromX` (`KismetMathLibrary.Normal` (- (`.Location` (`GameplayStatics.BreakHitResult` (`PlayerController.GetHitResultUnderCursorByChannel` (`GameplayStatics.GetPlayerController` 0) "TraceTypeQuery1" true))) (`self.K2_GetActorLocation`))))))
  (if (`self.Can_Fire_Cannon`)
    (`SceneComponent.K2_SetWorldRotation` (`self.AimArrow`) (`KismetMathLibrary.MakeRotator` 0.0 0.0 _returnvalue_yaw_2) false false)
    (`|ExecutionSequence`
      (:`then_0`
        (if (and (`self.faceUP`) (`self.aimUP`))
          (if (or (`self.faceDown`) (`self.faceLeft`) (`self.faceRight`))
            (set `self.Can_Fire_Cannon` false)
            (else
              (`|SpawnActorFromClass` "/Game/Blueprints/Player/Ammo/CannonBall_BP.CannonBall_BP_C" (`KismetMathLibrary.MakeTransform` (`SceneComponent.K2_GetComponentLocation` (`self.AimArrow`)) (`KismetMathLibrary.MakeRotator` 0.0 0.0 _returnvalue_yaw) (5.0 5.0 5.0)) "Undefined" "OverrideRootScale" :!label _label)
              (set `self.Can_Fire_Cannon` false)
              (if (>= _relativerotation_yaw -90.0)
                (`ActorComponent.Activate` (`self.RightPart`) true)
                (else
                  (`ActorComponent.Activate` (`self.LeftPart`) true)))))))
      (:`then_1`
        (if (and (`self.aimDown`) (`self.faceDown`))
          (goto _label)))
      (:`then_2`
        (if (and (`self.faceLeft`) (`self.AimLeft`))
          (goto _label)))
      (:`then_3`
        (if (and (`self.faceRight`) (`self.AimRight`))
          (goto _label))))))

(fn `ExplosiveShot`
  (bind (_relativerotation_roll _relativerotation_pitch _relativerotation_yaw) (`KismetMathLibrary.BreakRotator` (`SceneComponent.RelativeRotation` (`self.AimArrow`))))
  (bind (_returnvalue_roll _returnvalue_pitch _returnvalue_yaw) (`KismetMathLibrary.BreakRotator` (`KismetMathLibrary.MakeRotFromX` (`KismetMathLibrary.Normal` (- (`.Location` (`GameplayStatics.BreakHitResult` (`PlayerController.GetHitResultUnderCursorByChannel` (`GameplayStatics.GetPlayerController` 0) "TraceTypeQuery1" true))) (`self.K2_GetActorLocation`))))))
  (if (`self.Can_FIre_Explosive`)
    (`SceneComponent.K2_SetWorldRotation` (`self.AimArrow`) (`KismetMathLibrary.MakeRotator` 0.0 0.0 _returnvalue_yaw) false false)
    (`|ExecutionSequence`
      (:`then_0`
        (if (and (`self.faceUP`) (`self.aimUP`))
          (if (or (`self.faceDown`) (`self.faceLeft`) (`self.faceRight`))
            (set `self.Can_Fire_Cannon` false)
            (else
              (`|SpawnActorFromClass` "/Game/Blueprints/Player/Ammo/ExplosiveShot_BP.ExplosiveShot_BP_C" (`KismetMathLibrary.MakeTransform` (`SceneComponent.K2_GetComponentLocation` (`self.AimArrow`)) (`KismetMathLibrary.MakeRotator` 0.0)) "Undefined" "OverrideRootScale" :!label _label)
              (set `self.Can_FIre_Explosive` false)
              (if (>= _relativerotation_yaw -90.0)
                (`ActorComponent.Activate` (`self.RightPart`) true)
                (else
                  (`ActorComponent.Activate` (`self.LeftPart`) true)))))))
      (:`then_1`
        (if (and (`self.aimDown`) (`self.faceDown`))
          (goto _label)))
      (:`then_2`
        (if (and (`self.faceLeft`) (`self.AimLeft`))
          (goto _label)))
      (:`then_3`
        (if (and (`self.faceRight`) (`self.AimRight`))
          (goto _label))))))

(fn `UserConstructionScript`)