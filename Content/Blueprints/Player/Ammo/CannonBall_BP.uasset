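; CannonBall_BP is a cannonball ammo actor that trails smoke and removes itself on contact or after a short time.
; BeginPlay attaches a smoke emitter to Sphere1.
; A hit destroys the ball silently, while an overlap first spawns a musket-fire effect at its location.
; The lifetime comes from a two-second Delay started on Tick, and the graph contains no movement or damage logic.
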(event `self.ReceiveHit`
  (params (MyComp :type "PrimitiveComponent Object Reference") (Other :type "Actor Object Reference") (OtherComp :type "PrimitiveComponent Object Reference") (bSelfMoved :type Boolean) (HitLocation :type "Vector Structure") (HitNormal :type "Vector Structure") (NormalImpulse :type "Vector Structure") (Hit :type "HitResult Structure (by ref)"))
  (`self.K2_DestroyActor`))

(event `self.ReceiveBeginPlay`
  (`GameplayStatics.SpawnEmitterAttached` "/Game/Art/PolygonPirates/ParticleFX/P_FX_Smoke.P_FX_Smoke" (`self.Sphere1`)))

(event `self.ReceiveActorBeginOverlap`
  (params (OtherActor :type "Actor Object Reference"))
  (`GameplayStatics.SpawnEmitterAtLocation` "/Game/Art/PolygonPirates/ParticleFX/P_FX_MusketFire1.P_FX_MusketFire1" (`self.K2_GetActorLocation`))
  (`self.K2_DestroyActor`))

(event `self.ReceiveTick`
  (params (DeltaSeconds :type "Float (single-precision)"))
  (`KismetSystemLibrary.Delay` 2.0)
  (`self.K2_DestroyActor`))

(fn `UserConstructionScript`)