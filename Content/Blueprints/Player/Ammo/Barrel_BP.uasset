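; Barrel actor, filed under player ammo, that moves around its spawn point and disappears after a short lifetime or on contact with an enemy.
; BeginPlay caches the spawn location, and Tick plays a timeline whose Bob track is added to it to set the position.
; The timeline update also starts the delayed self-destruct, while overlapping an AI_Enemy destroys the barrel immediately, applying no damage.
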(event `self.ReceiveBeginPlay`
  (set `self.BarrelLoc` (`self.K2_GetActorLocation`)))

(event `self.ReceiveTick`
  (params (DeltaSeconds :type "Float (single-precision)"))
  (bind (_direction _bob) (`Timeline|Timeline_0`)
    (:`Update`
      (`self.K2_SetActorLocation` (+ _bob (`self.BarrelLoc`)))
      (`KismetSystemLibrary.Delay` 5.0)
      (`self.K2_DestroyActor`))))

(event `self.ReceiveActorBeginOverlap`
  (params (OtherActor :type "Actor Object Reference"))
  (cast `/Game/Blueprints/AI/AI_Enemy` OtherActor)
  (`self.K2_DestroyActor`))

(fn `UserConstructionScript`)