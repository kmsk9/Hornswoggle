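; Player ship Blueprint with force-driven sailing, HUD, island docking menus and a kill-count mission.
; Number keys select cannon, bar, explosive or barrel weapons with Delay-based cooldowns; shots aim at the cursor within a yaw limit, while barrels spawn at a drop point.
; Overlaps handle cannonball and rock damage plus gold pickups.
; Tick builds scurvy at sea, polls the mission and handles death: checkpoint respawn, leaving a shipwreck to reclaim lost gold.
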(event `Mission_01_Active`
  ;[1 0.9228 0] Comment
  (if (== (`self.BSKilledActive`) 2)
    (`self.Mission_01_Completed`)))

(event `Mission_01_Completed`
  ;[1 0.9228 0] Comment
  (set `self.Mission_01` false)
  (set `self.BSKilledActive` 0)
  (bind _returnvalue (`|CreateWidget` "/Game/Blueprints/UI/Missions_01_Complete.Missions_01_Complete_C" (`GameplayStatics.GetPlayerController` 0)))
  (`UserWidget.AddToViewport` _returnvalue 0))

(event `self.ReceiveBeginPlay`
  (set `PlayerController.bShowMouseCursor` true (`GameplayStatics.GetPlayerController` 0))
  (bind _returnvalue (`|CreateWidget` "/Game/Blueprints/UI/HUD.HUD_C"))
  (`UserWidget.AddToViewport` _returnvalue 0))

(event `self.ReceiveActorBeginOverlap`
  (params (OtherActor :type "Actor Object Reference"))
  (`|ExecutionSequence`
    (:`then_0`
      (if (`self.canBeDamaged`)
        (`|ExecutionSequence`
          (:`then_0`
            (cast `/Game/Blueprints/AI/Ammo/AI_CannonBall_BP` OtherActor))
          (:`then_1`
            (cast `/Game/Blueprints/AI/Ammo/AI_CannonBall_BP1` OtherActor :!label _label)))
        (set `self.Health` (- (`self.Health`) 5.0))
        (set `self.canBeDamaged` false :!label _label_2)
        (`KismetSystemLibrary.Delay` 0.2)
        (set `self.canBeDamaged` true)))
    (:`then_1`
      (bind _asgold_bp (cast `/Game/Blueprints/Extras/Gold_BP` OtherActor))
      (set `self.Gold` (+ (`self.Gold`) 100.0))
      (`self.K2_DestroyActor` _asgold_bp))
    (:`then_3`
      (goto _label))
    (:`then_4`
      (bind _asshipwreck (cast `/Game/Blueprints/Extras/Shipwreck` OtherActor))
      (set `self.Gold` (+ (`self.Gold`) (`self.GoldonDed`)))
      (`self.K2_DestroyActor` _asshipwreck))
    (:`then_5`
      (cast `/Game/Blueprints/IslandsHazards/Rocks` OtherActor)
      (set `self.Health` (- (`self.Health`) 25.0))
      (goto _label_2))))

(event `Key|One`
  (params (Key :type "Key Structure" :default "AnyKey"))
  ;[0 0.475 0.4112] Weapon Change
  (:`Pressed`
    (set `self.WeaponSelect` 1)))

(event `InputAxis|Move`
  (params (AxisValue :type "Float (single-precision)"))
  (bind (_returnvalue_roll _returnvalue_pitch _returnvalue_yaw) (`KismetMathLibrary.BreakRotator` (`SceneComponent.K2_GetComponentRotation` (`self.Ship`))))
  ;[0 0.02183 1] Movement
  (`PrimitiveComponent.AddForce` (`self.CapsuleComponent`) (* (* (`KismetMathLibrary.GetForwardVector` (`KismetMathLibrary.MakeRotator` _returnvalue_roll _returnvalue_pitch (+ _returnvalue_yaw 90.0))) AxisValue) (`self.Speed`)) "None" false))

(event `Key|Two`
  (params (Key :type "Key Structure" :default "AnyKey"))
  ;[0 0.475 0.4112] Weapon Change
  (:`Pressed`
    (set `self.WeaponSelect` 2)))

(event `Key|Three`
  (params (Key :type "Key Structure" :default "AnyKey"))
  ;[0 0.475 0.4112] Weapon Change
  (:`Pressed`
    (set `self.WeaponSelect` 3)))

(event `Key|Four`
  (params (Key :type "Key Structure" :default "AnyKey"))
  ;[0 0.475 0.4112] Weapon Change
  (:`Pressed`
    (set `self.WeaponSelect` 4)))

(event `InputAxis|Rotate`
  (params (AxisValue :type "Float (single-precision)"))
  (bind _returnvalue (* AxisValue (`GameplayStatics.GetWorldDeltaSeconds`) (`self.RotateSpeed`)))
  ;[0 0.02183 1] Movement
  (`|ExecutionSequence`
    (:`then_0`
      (`SceneComponent.K2_AddWorldRotation` (`self.Scene`) (`KismetMathLibrary.MakeRotator` 0.0 0.0 _returnvalue) false false))
    (:`then_1`
      (`SceneComponent.K2_AddWorldRotation` (`self.Scene`) (`KismetMathLibrary.MakeRotator` 0.0 0.0 _returnvalue) false false))))

(event `Key|E`
  (params (Key :type "Key Structure" :default "AnyKey"))
  ;[1 1 1] Open Menu
  (:`Pressed`
    (if (`self.CanDockMainIsland`)
      (bind _returnvalue (`|CreateWidget` "/Game/Blueprints/UI/Main_Island_MainMenuUI.Main_Island_MainMenuUI_C" (`GameplayStatics.GetPlayerController` 0)))
      (`UserWidget.AddToViewport` _returnvalue 0)
      (`WidgetBlueprintLibrary.SetInputMode_UIOnlyEx` (`GameplayStatics.GetPlayerController` 0))
      (elif (`self.CanDockEmptyIsland`)
        (bind _returnvalue_2 (`|CreateWidget` "/Game/Blueprints/UI/Empty_Island_MainMenuUI.Empty_Island_MainMenuUI_C" (`GameplayStatics.GetPlayerController` 0)))
        (`UserWidget.AddToViewport` _returnvalue_2 0)
        (`WidgetBlueprintLibrary.SetInputMode_UIOnlyEx` (`GameplayStatics.GetPlayerController` 0))))))

(event `InputAction|Shoot`
  (params (Key :type "Key Structure" :default "AnyKey"))
  ;[1 0 0] Shooting
  (:`Pressed`
    (`|ExecutionSequence`
      (:`then_0`
        (if (== (`self.WeaponSelect`) 1)
          (`self.CannonShot`)
          (`KismetSystemLibrary.Delay` 0.5)
          (set `self.Can_Fire_Cannon` true)))
      (:`then_1`
        (if (== (`self.WeaponSelect`) 2)
          (`self.BarShot`)
          (`KismetSystemLibrary.Delay` 2.0)
          (set `self.Can_Fire_Bar` true)))
      (:`then_2`
        (if (== (`self.WeaponSelect`) 3)
          (`self.ExplosiveShot`)
          (`KismetSystemLibrary.Delay` 0.3)
          (set `self.Can_FIre_Explosive` true)))
      (:`then_3`
        (if (== (`self.WeaponSelect`) 4)
          (`self.Barrel`)
          (`KismetSystemLibrary.Delay` 4.0)
          (set `self.Can_Fire_Barrel` true))))))

(event `self.ReceiveTick`
  (params (DeltaSeconds :type "Float (single-precision)"))
  ;[1 1 1] Event Tick
  (`|ExecutionSequence`
    (:`then_0`
      (if (`self.atSea`)
        (`KismetSystemLibrary.Delay` 3.0)
        (set `self.Scurvy` (+ (`self.Scurvy`) 1.0))))
    (:`then_1`
      (if (<= (`self.Health`) 0.0)
        (set `self.DeathPoint` (`self.K2_GetActorLocation`))
        (set `self.isDead` true)
        (set `self.GoldonDed` (`self.Gold`))
        (set `self.Gold` 0.0)
        (`self.K2_SetActorLocation` (`self.Checkpoint`))
        (set `self.Health` 100.0)))
    (:`then_2`
      (if (`self.isDead`)
        (`|SpawnActorFromClass` "/Game/Blueprints/Extras/Shipwreck.Shipwreck_C" (`KismetMathLibrary.MakeTransform` (`self.DeathPoint`)) "Undefined" "OverrideRootScale")
        (set `self.isDead` false)))
    (:`then_3`
      (if (`self.Mission_01`)
        (`self.Mission_01_Active`)))
    (:`then_4`
      (set `self.MissingHealth` (* (- (`self.Health`) 100.0) -1.0)))))

(fn `Barrel`
  (bind (_returnvalue_location _returnvalue_rotation) (`KismetMathLibrary.BreakTransform` (`SceneComponent.K2_GetComponentToWorld` (`self.Drop`))))
  (if (`self.Can_Fire_Barrel`)
    (`|SpawnActorFromClass` "/Game/Blueprints/Player/Ammo/Barrel_BP.Barrel_BP_C" (`KismetMathLibrary.MakeTransform` _returnvalue_location _returnvalue_rotation (0.5 0.5 0.5)) "Undefined" "OverrideRootScale")
    (set `self.Can_Fire_Barrel` false)))

(fn `BarShot`
  (bind (_returnvalue_roll _returnvalue_pitch _returnvalue_yaw) (`KismetMathLibrary.BreakRotator` (`SceneComponent.K2_GetComponentRotation` (`self.Tip`))))
  (bind (_returnvalue_roll_2 _returnvalue_pitch_2 _returnvalue_yaw_2) (`KismetMathLibrary.BreakRotator` (`KismetMathLibrary.MakeRotFromX` (`KismetMathLibrary.Normal` (- (`.Location` (`GameplayStatics.BreakHitResult` (`PlayerController.GetHitResultUnderCursorByChannel` (`GameplayStatics.GetPlayerController` 0) "TraceTypeQuery1" true))) (`self.K2_GetActorLocation`))))))
  (if (`self.Can_Fire_Bar`)
    (`SceneComponent.K2_SetWorldRotation` (`self.AimArrow`) (`KismetMathLibrary.MakeRotator` 0.0 0.0 _returnvalue_yaw_2) false false)
    (if (and (<= _returnvalue_yaw 120.0) (>= _returnvalue_yaw -120.0))
      (`|SpawnActorFromClass` "/Game/Blueprints/Player/Ammo/BarShot_BP.BarShot_BP_C" (`KismetMathLibrary.MakeTransform` (`SceneComponent.K2_GetComponentLocation` (`self.AimArrow`)) (`KismetMathLibrary.MakeRotator` 0.0 0.0 _returnvalue_yaw)) "Undefined" "OverrideRootScale")
      (set `self.Can_Fire_Bar` false))))

(fn `CannonShot`
  (bind (_returnvalue_roll _returnvalue_pitch _returnvalue_yaw) (`KismetMathLibrary.BreakRotator` (`SceneComponent.K2_GetComponentRotation` (`self.Tip`))))
  (bind (_returnvalue_roll_2 _returnvalue_pitch_2 _returnvalue_yaw_2) (`KismetMathLibrary.BreakRotator` (`KismetMathLibrary.MakeRotFromX` (`KismetMathLibrary.Normal` (- (`.Location` (`GameplayStatics.BreakHitResult` (`PlayerController.GetHitResultUnderCursorByChannel` (`GameplayStatics.GetPlayerController` 0) "TraceTypeQuery1" true))) (`self.K2_GetActorLocation`))))))
  (if (`self.Can_Fire_Cannon`)
    (`SceneComponent.K2_SetWorldRotation` (`self.AimArrow`) (`KismetMathLibrary.MakeRotator` 0.0 0.0 _returnvalue_yaw_2) false false)
    (if (and (<= _returnvalue_yaw 120.0) (>= _returnvalue_yaw -120.0))
      (`|SpawnActorFromClass` "/Game/Blueprints/Player/Ammo/CannonBall_BP.CannonBall_BP_C" (`KismetMathLibrary.MakeTransform` (`SceneComponent.K2_GetComponentLocation` (`self.AimArrow`)) (`KismetMathLibrary.MakeRotator` 0.0 0.0 _returnvalue_yaw)) "Undefined" "OverrideRootScale")
      (set `self.Can_Fire_Cannon` false))))

(fn `ExplosiveShot`
  (bind (_returnvalue_roll _returnvalue_pitch _returnvalue_yaw) (`KismetMathLibrary.BreakRotator` (`SceneComponent.K2_GetComponentRotation` (`self.Tip`))))
  (bind (_returnvalue_roll_2 _returnvalue_pitch_2 _returnvalue_yaw_2) (`KismetMathLibrary.BreakRotator` (`KismetMathLibrary.MakeRotFromX` (`KismetMathLibrary.Normal` (- (`.Location` (`GameplayStatics.BreakHitResult` (`PlayerController.GetHitResultUnderCursorByChannel` (`GameplayStatics.GetPlayerController` 0) "TraceTypeQuery1" true))) (`self.K2_GetActorLocation`))))))
  (if (`self.Can_FIre_Explosive`)
    (`SceneComponent.K2_SetWorldRotation` (`self.AimArrow`) (`KismetMathLibrary.MakeRotator` 0.0 0.0 _returnvalue_yaw_2) false false)
    (if (and (<= _returnvalue_yaw 120.0) (>= _returnvalue_yaw -120.0))
      (`|SpawnActorFromClass` "/Game/Blueprints/Player/Ammo/ExplosiveShot_BP.ExplosiveShot_BP_C" (`KismetMathLibrary.MakeTransform` (`SceneComponent.K2_GetComponentLocation` (`self.AimArrow`)) (`KismetMathLibrary.MakeRotator` 0.0 0.0 _returnvalue_yaw)) "Undefined" "OverrideRootScale")
      (set `self.Can_FIre_Explosive` false))))

(fn `UserConstructionScript`)