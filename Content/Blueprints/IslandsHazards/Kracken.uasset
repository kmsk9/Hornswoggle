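; Kraken island hazard that shoves a player who lingers inside its overlap area.
; Entering sets a hit flag and starts a short delay, while leaving clears the flag.
; If the flag is still set after the delay, it applies a smash-strength force to the player's capsule along the player's own forward vector and prints a debug string.
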(event `self.ReceiveActorBeginOverlap`
  (params (OtherActor :type "Actor Object Reference"))
  (bind _asplayer_bp_redo (cast `/Game/Blueprints/Player/Player_BP_Redo` OtherActor))
  (bind _output_get (set `self.canHit` true))
  (`KismetSystemLibrary.Delay` 2.0)
  (if _output_get
    (`PrimitiveComponent.AddForce` (`Character.CapsuleComponent` _asplayer_bp_redo) (* (`SceneComponent.GetForwardVector` (`Character.CapsuleComponent` _asplayer_bp_redo)) (`self.SmashStrength`)) "None" false)
    (`KismetSystemLibrary.PrintString` "Hello")))

(event `self.ReceiveActorEndOverlap`
  (params (OtherActor :type "Actor Object Reference"))
  (cast `/Game/Blueprints/Player/Player_BP_Redo` OtherActor)
  (set `self.canHit` false))

(fn `UserConstructionScript`)